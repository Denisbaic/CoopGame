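; BP_Projectile is a timed explosive projectile that detonates after a fixed delay, with no impact logic in its graph.
; On BeginPlay it launches along the Sphere's forward vector using the ProjectileMovement component's initial speed.
; When the timer ends it applies full radial damage, ignoring itself and its owner, and draws a debug sphere if damage landed.
; It then spawns an explosion particle effect and destroys itself.
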(event EventBeginPlay
  (bind _returnvalue (Components|GetOwner))
  (bind _self self)
  (bind _projectilemovement (Variables|Default|GetProjectileMovement))
  (bind _sphere (Variables|Default|GetSphere))
  (bind _returnvalue_2 (Transformation|GetWorldLocation _sphere))
  (Variables|/Script/Engine.MovementComponent|SetVelocity _projectilemovement (* (Math|Rotator|GetRotationXVector (Transformation|GetWorldRotation (Variables|Default|GetSphere))) (Variables|/Script/Engine.ProjectileMovementComponent|GetInitialSpeed _projectilemovement)))
  (Components|Activation|SetActive (Variables|Default|GetProjectileMovement) true false)
  (Utilities|FlowControl|Delay 3.0)
  (bind _returnvalue_3 (Game|Damage|ApplyRadialDamage 3e+01 _returnvalue_2 3e+02 0 (Utilities|Array|MakeArray _returnvalue _self) _self (Game|GetInstigatorController _returnvalue) true "ECC_PhysicsBody"))
  (if _returnvalue_3
    (Rendering|Debug|DrawDebugSphere _returnvalue_2 3e+02 12 "(R=0.000000,G=0.833200,B=1.000000,A=1.000000)" 3.0 3.0))
  (Effects|SpawnEmitteratLocation "/Game/WeaponEffects/Explosion/P_Explosion.P_Explosion" (Transformation|GetActorLocation))
  (Actor|DestroyActor))

(event Collision|EventActorBeginOverlap
  (params (OtherActor :type Actor%20Object%20Reference)))

(event EventTick
  (params (DeltaSeconds :type Float%20%28single-precision%29)))

(fn ConstructionScript)